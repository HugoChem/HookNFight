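; BP_HookNFightCharacter3 is a modular player character Blueprint with highlight feedback for targets and immunity.
; Its construction script leader-poses the body parts to Mesh and applies one shared dynamic material to all parts, BaseMesh and the sword.
; The second material loop also pulls axis inversion and effect volume from Main_Game_Instance.
; Target highlights are forwarded as messages to the target, while immunity highlights recolor the character through that material.
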(event EventTargetHighlight
  (params (target2 :type Actor%20Object%20Reference) (state :type Boolean))
  ;[1 1 1] TargetHighLight
  (Class|BPIHighLight|Highlight(Message) target2 state))

(event EventImmuneHighlight
  (params (state :type Boolean))
  ;[1 1 1] ImmuneHighLight
  (CallFunction|HighlightModularCharacter (Variables|Default|GetDynamicMaterial) (Variables|Default|GetimmuneHighLightColor) (Variables|Default|GetHighLightValue) (Variables|Default|GetAdditionalStuffs) (Variables|Default|GetFullBody) state))

(fn ConstructionScript
  (bind _returnvalue (Game|GetGameInstance))
  (bind _asmain_game_instance (Utilities|Casting|CastToMain_Game_Instance _returnvalue))
  ;[1 1 1] Constructor
  (bind _returnvalue_2 (Rendering|Material|CreateDynamicMaterialInstance (Rendering|Material|GetMaterial (Variables|Default|GetbaseMesh) 0) "None" :!class /Script/Engine.KismetMaterialLibrary))
  (Variables|Default|SetDynamicMaterial _returnvalue_2)
  (Variables|Default|SetBodyPart (Utilities|Array|MakeArray (Variables|Default|GetHair) (Variables|Default|GetGlove) (Variables|Default|GetShoe) (Variables|Default|GetHeadGears) (Variables|Default|GetShoulderPad) (Variables|Default|GetBelt) (Variables|Default|GetFace)))
  (Class|SkinnedMeshComponent|SetMasterPoseComponent (Variables|Default|GetBodyPart) (Variables|Character|GetMesh) false)
  (bind _output_get (Variables|Default|SetFullBody (Variables|Default|GetBodyPart)))
  (Utilities|Array|Add _output_get (Variables|Character|GetMesh))
  (Variables|Default|SetAdditionalStuffs (Utilities|Array|MakeArray (Variables|Default|GetbaseMesh) (Variables|Default|GetSword01SM)))
  (for _array_element (Variables|Default|GetFullBody)
    (Rendering|Material|SetMaterial _array_element 0 (Variables|Default|GetDynamicMaterial)))
  (for _array_element_2 (Variables|Default|GetAdditionalStuffs)
    (Rendering|Material|SetMaterial _array_element_2 0 (Variables|Default|GetDynamicMaterial))
    (Variables|Default|SetXAxisInverted (Variables|/Game/w_nardone/Game/Main_Game_Instance.Main_Game_Instance_C|GetInst_X_Axis_Inverted _asmain_game_instance))
    (Variables|Default|SetYAxisInverted (Variables|/Game/w_nardone/Game/Main_Game_Instance.Main_Game_Instance_C|GetInst_Y_Axis_Inverted _asmain_game_instance))
    (Class|CharacterBase|SetEffectVolume (Variables|/Game/w_nardone/Game/Main_Game_Instance.Main_Game_Instance_C|GetInst_Effect_Volume _asmain_game_instance))))