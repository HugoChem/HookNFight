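; Blueprint for an AI control director unit, handling music, player healing and victory as its phases change.
; Phase start plays one track, then another after a short delay; phase end switches music and restores the player's Life to MaxLife.
; When all directors are shut down, it waits briefly and opens the VictoryScreen level.
; The construction script creates a dynamic glow material instance on MainSphere.
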(event EventDirectorEndedPhase
  (bind _returnvalue (Game|GetPlayerCharacter 0))
  (bind _asbp_hook_nfight_character_3 (Utilities|Casting|CastToBP_HookNFightCharacter3 _returnvalue))
  (CallFunction|PlayMusic (.AsMain%20Game%20Instance (Utilities|Casting|CastToMain_Game_Instance (Game|GetGameInstance))) "/Game/w_nardone/Game/Sounds/Musique/Goliath_s_Foe.Goliath_s_Foe" 1.0 0.0)
  (Variables|/Script/HookNFight.CharacterBase|Setlife _asbp_hook_nfight_character_3 (Variables|/Script/HookNFight.HookNFightCharacter|GetmaxLife _asbp_hook_nfight_character_3)))

(event EventDirectorShuttedDown
  (params (AllDirectorsShutDown :type Boolean))
  (if AllDirectorsShutDown
    (Utilities|FlowControl|Delay 5.0)
    (Game|OpenLevel(byName) "VictoryScreen")))

(event EventDirectorBeganPhase
  (bind _returnvalue (Game|GetGameInstance))
  (bind _asmain_game_instance (Utilities|Casting|CastToMain_Game_Instance _returnvalue))
  (CallFunction|PlayMusic _asmain_game_instance "/Game/w_nardone/Game/Sounds/Musique/5_Julie_ting_.5_Julie_ting_" 1.0 0.0)
  (Utilities|FlowControl|Delay 2.2)
  (CallFunction|PlayMusic _asmain_game_instance "/Game/w_nardone/Game/Sounds/Musique/5_Julie__music_wav.5_Julie__music_wav" 1.0 0.0))

(fn ConstructionScript
  (Rendering|Material|CreateDynamicMaterialInstance (Variables|Default|GetMainSphere) 0 "/Game/h_chemouny/Materials/MI_Glowy.MI_Glowy" "None" :!class /Script/Engine.PrimitiveComponent))