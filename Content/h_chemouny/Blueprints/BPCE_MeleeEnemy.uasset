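; Melee enemy character that supports highlighting as a target of the player's HookNFightCharacter.
; BeginPlay puts a dynamic material instance on the mesh, which the Highlight event uses to toggle the highlight.
; Tick turns the highlight off when this enemy is the player's target but has not been rendered recently.
; Switching the highlight off also calls ChangeCharacterTarget, so an off-screen enemy triggers a target change.
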(event EventBeginPlay
  ;[1 1 1] Constructor
  (bind _returnvalue (Rendering|Material|CreateDynamicMaterialInstance (Rendering|Material|GetMaterial (Variables|Character|GetMesh) 0) "None" :!class /Script/Engine.KismetMaterialLibrary))
  (bind _output_get (Variables|Default|SetDynamicMaterial _returnvalue))
  (Rendering|Material|SetMaterial (Variables|Character|GetMesh) 0 _output_get))

(event EventTick
  (params (DeltaSeconds :type Float%20%28single-precision%29))
  (bind _returnvalue (Class|Actor|WasRecentlyRendered 0.2))
  ;[1 1 1] Tick
  (bind _ashook_nfight_character (Utilities|Casting|CastToHookNFightCharacter (Game|Player|GetPlayerPawn 0)))
  (if (== (Variables|/Script/HookNFight.HookNFightCharacter|Gettarget _ashook_nfight_character) self)
    (if (not _returnvalue)
      (CallFunction|Highlight _returnvalue))))

(event EventHighlight
  (params (State :type Boolean))
  ;[1 1 1] Highlight
  (CallFunction|HighlightOneMeshCharacter (Variables|Default|GetDynamicMaterial) (Variables|Default|GetHighlightValue) (Variables|Default|GetHighlightColor) State)
  (if (not State)
    (CallFunction|ChangeCharacterTarget)))

(fn ConstructionScript)